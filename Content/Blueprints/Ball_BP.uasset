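; Ball actor for a paddle-and-ball game, reset to a fixed spot with a randomly angled direction when BallGameMode signals play start.
; In one game state, Tick moves it by a swept XY offset, unscaled by delta time, and reflects it off impact normals.
; Paddle hits skew the bounce by the paddle's axis input and a MinX bias.
; Other hit actors implementing BallHitInterface receive a HitByBall message.
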(event `self.ReceiveBeginPlay`
  (bind _asball_game_mode (cast `/Game/Blueprints/BallGameMode` (`GameplayStatics.GetGameMode`)))
  (add `/Game/Blueprints/BallGameMode.StartPlaying` _asball_game_mode (delegate `BallStartPlaying`)))

(event `BallStartPlaying`
  (`self.ResetBallPosition`))

(event `self.ReceiveTick`
  (params (DeltaSeconds :type "Float (single-precision)"))
  (bind _asball_game_mode (cast `/Game/Blueprints/BallGameMode` (`GameplayStatics.GetGameMode`)))
  (if (`|EnumEquality` (`/Game/Blueprints/BallGameMode.StateOfTheGame` _asball_game_mode) "NewEnumerator5")
    (bind _sweephitresult (`self.K2_AddActorWorldOffset` (`KismetMathLibrary.MakeVector` (.x (* (`self.Direction`) (`self.Speed`))) (.y (* (`self.Direction`) (`self.Speed`)))) true))
    (bind (_bblockinghit _binitialoverlap _time _distance _location _impactpoint _normal _impactnormal _physmat _hitactor) (`GameplayStatics.BreakHitResult` _sweephitresult))
    (bind _aspaddle (cast `/Game/Blueprints/Paddle` _hitactor)
      (:`then`
        (bind _returnvalue (`KismetMathLibrary.GetReflectionVector` (`self.Direction`) _impactnormal))
        (set `self.Direction` (`KismetMathLibrary.Normal` (`KismetMathLibrary.MakeVector` (+ (.x (`KismetMathLibrary.Normal` (`KismetMathLibrary.MakeVector` (.x _returnvalue) (+ (* (`/Game/Blueprints/Paddle.AxisValue` _aspaddle) 5.0) (.y _returnvalue)) (.z _returnvalue)))) (`self.MinX`)) (.y (`KismetMathLibrary.Normal` (`KismetMathLibrary.MakeVector` (.x _returnvalue) (+ (* (`/Game/Blueprints/Paddle.AxisValue` _aspaddle) 5.0) (.y _returnvalue)) (.z _returnvalue)))) (.z (`KismetMathLibrary.Normal` (`KismetMathLibrary.MakeVector` (.x _returnvalue) (+ (* (`/Game/Blueprints/Paddle.AxisValue` _aspaddle) 5.0) (.y _returnvalue)) (.z _returnvalue))))))))
      (:`CastFailed`
        (set `self.Direction` _returnvalue)
        (if (`KismetSystemLibrary.DoesImplementInterface` _hitactor "/Game/Blueprints/BallHitInterface.BallHitInterface_C")
          (message `/Game/Blueprints/BallHitInterface.HitByBall` _hitactor))))))

(fn `ResetBallPosition`
  (`self.K2_SetActorLocation` (-400.0 0.0 30.0))
  (set `self.Direction` (`KismetMathLibrary.Normal` (`KismetMathLibrary.MakeVector` 1.0 (`KismetMathLibrary.RandomFloatInRange` -1.0 1.0)))))

(fn `UserConstructionScript`)