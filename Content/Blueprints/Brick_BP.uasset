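; Brick actor for a ball-and-brick game that loses a hit point each time the ball hits it and is destroyed when none remain.
; On BeginPlay it creates a BrickNumber widget linked back to itself and shows it on its NumberComponent.
; Each hit plays a sound, and destruction decrements the game mode's brick count and increments the player score on the game instance.
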(event `self.ReceiveBeginPlay`
  (bind _returnvalue (`|CreateWidget` "/Game/HUD/BrickNumber_WBP.BrickNumber_WBP_C"))
  (set `/Game/HUD/BrickNumber_WBP.RefToBrick` self _returnvalue)
  (`WidgetComponent.SetWidget` (`self.NumberComponent`) _returnvalue))

(event `/Game/Blueprints/BallHitInterface.HitByBall`
  (`self.DecrementHitPoints`)
  (`GameplayStatics.PlaySound2D` null 1.0 1.0 0.0 null null))

(fn `DecrementHitPoints`
  (if (<= (- (`self.HitPoints`) 1) 0)
    (bind _asball_game_mode (cast `/Game/Blueprints/BallGameMode` (`GameplayStatics.GetGameMode`)))
    (`/Game/Blueprints/BallGameMode.DecrementBrickCount` _asball_game_mode)
    (bind _asball_game_instance (cast `/Game/Blueprints/BallGameInstance` (`GameplayStatics.GetGameInstance`)))
    (`/Engine/EditorBlueprintResources/StandardMacros.IncrementInt` (`/Game/Blueprints/BallGameInstance.PlayerScore` _asball_game_instance)
      (:`  `
        (`self.K2_DestroyActor`)))
    (else
      (`/Engine/EditorBlueprintResources/StandardMacros.DecrementInt` (`self.HitPoints`)))))

(fn `UserConstructionScript`)